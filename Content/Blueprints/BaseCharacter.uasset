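; BaseCharacter is a character Blueprint that manages health (Salud), pain sounds and death.
; AnyDamage adds the damage value as a signed delta to clamped health, then updates IsDead.
; Survivors play a random pain sound; death plays the last sound once, ignores WorldDynamic and Pawn collisions, detaches the controller and destroys the actor after a delay.
; Functions expose health values and update the InfoBar widget's health bar.
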(event Custom|CalculeSalud
  (params (Delta :type Float%20%28single-precision%29))
  (bind _capsulecomponent (Variables|Collision|GetCapsuleComponent))
  (Variables|Default|SetSalud (Math|Float|Clamp(Float) (+ Delta (Variables|Default|GetSalud)) 0.0 (Variables|Default|GetSaludMax)))
  (CallFunction|CalculeDead)
  (if (Variables|Default|GetbIsDead)
    (Utilities|FlowControl|DoOnce false :!label _label
      (:Completed
        (Utilities|Auuu (Utilities|Array|LastIndex (Variables|Default|GetArrayPainAU)))
        (Collision|SetCollisionResponsetoChannel _capsulecomponent "ECC_WorldDynamic" "ECR_Ignore") ; De esta forma el enemgo caído ignora los proyectiles
        (Collision|SetCollisionResponsetoChannel _capsulecomponent "ECC_Pawn" "ECR_Ignore") ; Y al Hero, aunque podría ser útil que los cuerpos entorpecieran el mvto, poner block entonces
        (Class|Pawn|DetachfromControllerPendingDestroy)
        (Utilities|FlowControl|Delay 1.5)
        (Actor|DestroyActor)))
    (else
      (Utilities|Auuu)
      (goto _label Reset))))

(event Custom|CalculeDead
  (if (<= (Variables|Default|GetSalud) 0.0)
    (Variables|Default|SetbIsDead true)
    (else
      (Variables|Default|SetbIsDead false))))

(event EventBeginPlay)

(event EventTick
  (params (DeltaSeconds :type Float%20%28single-precision%29)))

(event Game|Damage|EventAnyDamage
  (params (Damage :type Float%20%28single-precision%29) (DamageType :type Damage%20Type%20Object%20Reference) (InstigatedBy :type Controller%20Object%20Reference) (DamageCauser :type Actor%20Object%20Reference))
  (CallFunction|CalculeSalud Damage))

(fn ConstructionScript)

(fn GetHealth
  (return (Variables|Default|GetSalud)))

(fn GetMaxHealth
  (return (Variables|Default|GetSaludMax)))

(fn ShowHealth
  (params (CurrentHelth :type Float%20%28single-precision%29) (MaxHealth :type Float%20%28single-precision%29))
  (bind _ashealth_base_character (Utilities|Casting|CastToHealthBaseCharacter (UserInterface|GetUserWidgetObject (Variables|Default|GetInfoBar))))
  (Progress|SetPercent (Variables|/Game/UI/HealthBaseCharacter.HealthBaseCharacter_C|GetHealthBar _ashealth_base_character) (/ CurrentHelth MaxHealth)))