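; Prototype thrown hammer actor for BP_AxeKid, moved by a timeline rather than physics or projectile movement.
; Tira plays the timeline, offsetting the mesh from its BeginPlay location along the owner's ArrowToSpawn forward vector, re-read each update, without sweeping.
; Recoge reverses the timeline to pull the hammer back.
; The actor destroys itself shortly after the timeline finishes.
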(event Custom|Tira
  (bind (_direction _forcelaunchhammer _movement) (Timeline|Timeline_0 Play)
    (:Update
      (Transformation|SetWorldLocation (Variables|Default|GetStaticMesh) (+ (Variables|Default|GetInitialCubeLocation) (* (Math|Vector|GetForwardVector (Transformation|GetWorldRotation (Variables|/Game/Blueprints/Heros/BP_AxeKid.BP_AxeKid_C|GetArrowToSpawn (.AsBP%20Axe%20Kid (Utilities|Casting|CastToBP_AxeKid (Components|GetOwner)))))) _forcelaunchhammer)) false false))
    (:Finished
      (Utilities|FlowControl|Delay 0.2)
      (Actor|DestroyActor))))

(event Custom|Recoge
  (bind (_direction _forcelaunchhammer _movement) (Timeline|Timeline_0 Reverse)
    (:Update
      (Transformation|SetWorldLocation (Variables|Default|GetStaticMesh) (+ (Variables|Default|GetInitialCubeLocation) (* (Math|Vector|GetForwardVector (Transformation|GetWorldRotation (Variables|/Game/Blueprints/Heros/BP_AxeKid.BP_AxeKid_C|GetArrowToSpawn (.AsBP%20Axe%20Kid (Utilities|Casting|CastToBP_AxeKid (Components|GetOwner)))))) _forcelaunchhammer)) false false))
    (:Finished
      (Utilities|FlowControl|Delay 0.2)
      (Actor|DestroyActor))))

(event EventBeginPlay
  (Variables|Default|SetInitialCubeLocation (Transformation|GetWorldLocation (Variables|Default|GetStaticMesh)))
  (Utilities|FlowControl|Delay 8.0))

(fn ConstructionScript)