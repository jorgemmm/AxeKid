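; BP_Enemy is an enemy character, filed under ZombieSlime, that damages the BP_AxeKid hero on contact.
; DamageBox overlap starts a looping timer that applies BaseDamage at a DPS-based rate, and end overlap clears it.
; While alive, Tick calls ShowHealth unless IsHeroNearToUpdateHealth returns true.
; Despite its name, that check flags distances of 1000 or more, measured from the enemy's own location to its InfoBar.
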(event OnComponentBeginOverlap(DamageBox)
  (params (OverlappedComponent :type Primitive%20Component%20Object%20Reference) (OtherActor :type Actor%20Object%20Reference) (OtherComp :type Primitive%20Component%20Object%20Reference) (OtherBodyIndex :type Integer) (bFromSweep :type Boolean) (SweepResult :type Hit%20Result%20Structure%20%28by%20ref%29))
  (if (!= OtherActor self)
    (bind _asbp_axe_kid (Utilities|Casting|CastToBP_AxeKid OtherActor))
    (Variables|Default|SetHero _asbp_axe_kid)
    (Utilities|Time|SetTimerbyFunctionName 0 "DamageToHero" (/ 1.0 (Variables|Default|GetDPS)) true)))

(event OnComponentEndOverlap(DamageBox)
  (params (OverlappedComponent :type Primitive%20Component%20Object%20Reference) (OtherActor :type Actor%20Object%20Reference) (OtherComp :type Primitive%20Component%20Object%20Reference) (OtherBodyIndex :type Integer))
  (if (== OtherActor (Variables|Default|GetHero))
    (Utilities|Time|ClearTimerbyFunctionName 0 "DamageToHero")))

(event Custom|DamageToHero
  (Game|Damage|ApplyDamage (Variables|Default|GetHero) (Variables|Default|GetBaseDamage) (Game|GetInstigatorController) self))

(event EventBeginPlay
  (Variables|/Script/Engine.CharacterMovementComponent|SetMaxWalkSpeed (Variables|Character|GetCharacterMovement) 2e+02))

(event Collision|EventActorBeginOverlap
  (params (OtherActor :type Actor%20Object%20Reference)))

(event EventTick
  (params (DeltaSeconds :type Float%20%28single-precision%29))
  (|CallParentFunction DeltaSeconds)
  (if (not (Variables|Default|GetbIsDead)) ; Si Zombie is dead No pasamos
    (bind _returnvalue (Utilities|IsHeroNeartoUpdateHealth)
      (:bSuccess
        (if (not _returnvalue) ; Si hero muy lejano no hacemos nada
          (CallFunction|ShowHealth (Variables|Default|GetSalud) (Variables|Default|GetSaludMax)))))))

(fn ConstructionScript)